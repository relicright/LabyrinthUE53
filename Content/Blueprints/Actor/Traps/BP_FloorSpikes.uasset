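; Floor spike trap that deals physical damage to an actor overlapping its Box through the Gameplay Ability System.
; An overlap while armed disarms the trap, applies GE_Damage, then re-arms after a fixed delay.
; The overlapping actor's ability system component serves as both damage source and target.
; Debug prints remain, along with an unexecuted ApplyEffectToTarget branch.
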(event `self.Box.OnComponentBeginOverlap`
  (params (OverlappedComponent :type "PrimitiveComponent Object Reference") (OtherActor :type "Actor Object Reference") (OtherComp :type "PrimitiveComponent Object Reference") (OtherBodyIndex :type Integer) (bFromSweep :type Boolean) (SweepResult :type "HitResult Structure (by ref)"))
  (bind _returnvalue (`AbilitySystemBlueprintLibrary.GetAbilitySystemComponent` OtherActor))
  (if (`self.IsArmed?`)
    (set `self.IsArmed?` false)
    (`LabyrinthAbilitySystemLibrary.ApplyDamageEffect` (make `DamageEffectParams` self "/Game/Blueprints/AbilitySystem/GE_Damage.GE_Damage_C" _returnvalue _returnvalue 100.0 1.0 (struct :`TagName` "Damage.Physical")))
    (`KismetSystemLibrary.Delay` 4.0)
    (set `self.IsArmed?` true)
    (`KismetSystemLibrary.PrintString` "Hello")
    (else
      (`KismetSystemLibrary.PrintString` "Not Set"))))

(event `self.Box.OnBeginCursorOver`
  (params (TouchedComponent :type "PrimitiveComponent Object Reference"))
  (`KismetSystemLibrary.PrintString` "asdasdsad"))

(fn `UserConstructionScript`
  (`parent.UserConstructionScript`))