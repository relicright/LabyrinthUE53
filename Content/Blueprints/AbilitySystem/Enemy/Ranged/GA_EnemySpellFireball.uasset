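; Enemy gameplay ability for a ranged fireball attack that spawns a projectile at the avatar's combat target.
; On activation it turns the avatar toward the target and plays the Lich left-hand attack montage, with play rate scaled by an attribute noted as Dex.
; The first attack montage event spawns the projectile from the left-hand socket toward the target's current location.
; The random montage pick is unused, and EndAbility is never reached.
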(event `self.K2_ActivateAbility`
  (bind _returnvalue (`self.GetAvatarActorFromActorInfo`))
  (bind _returnvalue_2 (`self.GetAvatarActorFromActorInfo`))
  (bind _returnvalue_3 (`BlueprintGameplayTagLibrary.MakeLiteralGameplayTag` (struct :`TagName` "CombatSocket.LeftHand")))
  ;[0.09549 0.4203 1] Get Target and Facing Rotation
  (bind _returnvalue_4 (message `EnemyInterface.GetCombatTarget` _returnvalue_2))
  (bind _ascombat_interface (cast `CombatInterface` _returnvalue_2))
  (message `CombatInterface.UpdateFacingTarget` (`KismetSystemLibrary.Conv_InterfaceToObject` _ascombat_interface) (`Actor.K2_GetActorLocation` _returnvalue_4))
  ;[0.1345 0.09615 1] Get montages and pick one from random
  (bind _returnvalue_5 (message `CombatInterface.GetAttackMontages` (`self.GetAvatarActorFromActorInfo`)))
  (bind _output_get (set `self.TaggedMontage` (`self.GetRandomTaggedMontageFromArray` _returnvalue_5)))
  (`AbilityTask_PlayMontageAndWait.CreatePlayMontageAndWaitProxy` "None" "/Game/Assets/Animations/Character/Lich/AM_Lich_Attack_Left.AM_Lich_Attack_Left" (+ (/ (`.ReturnValue` (`AbilitySystemComponent.GetGameplayAttributeValue` (`AbilitySystemBlueprintLibrary.GetAbilitySystemComponent` (`self.GetAvatarActorFromActorInfo`)) (struct :`AttributeName` "Dexterity" :`Attribute` "/Script/LabyrinthUE53.LabyrinthAttributeSet:Dexterity" :`AttributeOwner` "/Script/CoreUObject.Class'/Script/LabyrinthUE53.LabyrinthAttributeSet'"))) 100.0) 1.0)
    (:`then`
      (`AbilityTask_WaitGameplayEvent.WaitGameplayEvent` (struct :`TagName` "Montage.Attack.1") null true
        (:`EventReceived`
          (message `CombatInterface.GetCombatSocketLocation` _returnvalue _returnvalue_3)
          (bind _returnvalue_6 (message `EnemyInterface.GetCombatTarget` _returnvalue))
          (`self.SpawnProjectile` (`Actor.K2_GetActorLocation` _returnvalue_6) _returnvalue_3 (`self.ShouldOverridePitch`) (`self.PitchOverride`)))))))