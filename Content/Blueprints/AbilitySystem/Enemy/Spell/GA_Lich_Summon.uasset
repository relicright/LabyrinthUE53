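; Lich enemy gameplay ability for a summon spell, apparently unfinished: it plays the cast but spawns nothing.
; On activation it turns the avatar toward its combat target through CombatInterface and plays the summon montage.
; A one-shot wait for the Montage.Attack.1 gameplay event then fetches the left-hand socket location and combat target, without using either.
; Montage stop and EndAbility nodes are unconnected, so the graph never ends the ability.
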(event `self.K2_ActivateAbility`
  (bind _returnvalue (`self.GetAvatarActorFromActorInfo`))
  (bind _returnvalue_2 (`self.GetAvatarActorFromActorInfo`))
  ;[0.09549 0.4203 1] Get Target and Facing Rotation
  (bind _returnvalue_3 (message `EnemyInterface.GetCombatTarget` _returnvalue_2))
  (bind _ascombat_interface (cast `CombatInterface` _returnvalue_2))
  (message `CombatInterface.UpdateFacingTarget` (`KismetSystemLibrary.Conv_InterfaceToObject` _ascombat_interface) (`Actor.K2_GetActorLocation` _returnvalue_3))
  ;[0.1345 0.09615 1] Get montages and pick one from random
  (`AbilityTask_PlayMontageAndWait.CreatePlayMontageAndWaitProxy` "None" "/Game/Assets/Animations/Character/Lich/AM_Lich_Summon.AM_Lich_Summon"
    (:`then`
      (`AbilityTask_WaitGameplayEvent.WaitGameplayEvent` (struct :`TagName` "Montage.Attack.1") null true
        (:`EventReceived`
          (message `CombatInterface.GetCombatSocketLocation` _returnvalue (`BlueprintGameplayTagLibrary.MakeLiteralGameplayTag` (struct :`TagName` "CombatSocket.LeftHand")))
          (bind _returnvalue_4 (message `EnemyInterface.GetCombatTarget` _returnvalue)))))))