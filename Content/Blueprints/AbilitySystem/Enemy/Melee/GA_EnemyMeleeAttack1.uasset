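; Enemy melee attack gameplay ability that faces the combat target and plays a random tagged attack montage at a Dexterity-scaled rate.
; The montage's gameplay event triggers a sphere check for live players at the tagged combat socket.
; A blocking player stops the montage and triggers the enemy's hit react, while an unblocked one takes damage with overridden knockback, limited to one hit per activation.
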(event `self.K2_ActivateAbility`
  (bind _returnvalue (`self.GetAvatarActorFromActorInfo`))
  (bind _returnvalue_2 (`self.GetAvatarActorFromActorInfo`))
  (set `self.HasHitTarget` false)
  ;[0.09549 0.4203 1] Get Target and Facing Rotation
  (bind _returnvalue_3 (message `EnemyInterface.GetCombatTarget` _returnvalue_2))
  (bind _ascombat_interface (cast `CombatInterface` _returnvalue_2))
  (message `CombatInterface.UpdateFacingTarget` (`KismetSystemLibrary.Conv_InterfaceToObject` _ascombat_interface) (`Actor.K2_GetActorLocation` _returnvalue_3))
  ;[0.1345 0.09615 1] Get montages and pick one from random
  (bind _returnvalue_4 (message `CombatInterface.GetAttackMontages` (`self.GetAvatarActorFromActorInfo`)))
  (bind _output_get (set `self.TaggedMontage` (`self.GetRandomTaggedMontageFromArray` _returnvalue_4)))
  (bind (_montage _montagetag _sockettag) (break `TaggedMontage` _output_get))
  (`AbilityTask_PlayMontageAndWait.CreatePlayMontageAndWaitProxy` "None" _montage (+ (/ (`.ReturnValue` (`AbilitySystemComponent.GetGameplayAttributeValue` (`AbilitySystemBlueprintLibrary.GetAbilitySystemComponent` (`self.GetAvatarActorFromActorInfo`)) (struct :`AttributeName` "Dexterity" :`Attribute` "/Script/LabyrinthUE53.LabyrinthAttributeSet:Dexterity" :`AttributeOwner` "/Script/CoreUObject.Class'/Script/LabyrinthUE53.LabyrinthAttributeSet'"))) 100.0) 1.0)
    (:`then`
      ;[1 0.9225 0.3229] Wait for Gameplay Event from Montage and Check Surrounding Targets
      (`AbilityTask_WaitGameplayEvent.WaitGameplayEvent` _montagetag null
        (:`EventReceived`
          (bind _returnvalue_5 (message `CombatInterface.GetCombatSocketLocation` _returnvalue _sockettag))
          (bind _output_get_2 (set `self.CombatSocketLocation` _returnvalue_5))
          (bind _outoverlappingactors (`LabyrinthAbilitySystemLibrary.GetLivePlayersWithinRadius` _returnvalue (`|MakeArray` _returnvalue) 90.0 _output_get_2))
          (for _array_element _outoverlappingactors
            (if (`self.HasHitTarget`)
              _
              (elif (`GameplayTagAssetInterface.HasMatchingGameplayTag` (`AbilitySystemBlueprintLibrary.GetAbilitySystemComponent` _array_element) (struct :`TagName` "Player.Block"))
                ;[1 0.1521 0.8232 1 20] Blocked Attack Resulting in a Hit React
                (`self.MontageStop` -1.0)
                (`AbilitySystemComponent.TryActivateAbilitiesByTag` (`AbilitySystemBlueprintLibrary.GetAbilitySystemComponent` (`self.GetAvatarActorFromActorInfo`)) (`BlueprintGameplayTagLibrary.MakeGameplayTagContainerFromArray` (`|MakeArray` (`BlueprintGameplayTagLibrary.MakeLiteralGameplayTag` (struct :`TagName` "Effects.HitReact")))) true)
                (else
                  ;[1 0.08141 0.05157 1 20] Not Blocked hit Resulting in Damage
                  (`LabyrinthAbilitySystemLibrary.ApplyDamageEffect` (`self.MakeDamageEffectParamsFromClassDefaults` _array_element (0.0 0.0 0.0) true (0.0 0.0 10000.0)))
                  (set `self.HasHitTarget` true))))))))
    (:`OnCompleted`
      ;[0 1 0.004274] End Ability
      (`self.K2_EndAbility` :!label _label))
    (:`OnInterrupted`
      (goto _label))
    (:`OnCancelled`
      (goto _label))))

(event `self.K2_OnEndAbility`
  (params (bWasCancelled :type Boolean))
  (`self.MontageStop` -1.0))