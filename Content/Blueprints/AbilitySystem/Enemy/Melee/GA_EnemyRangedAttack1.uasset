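; Gameplay ability for an enemy ranged attack that fires a projectile at the avatar's combat target.
; On activation it turns the avatar toward the target and plays a random tagged attack montage, sped up by an attribute commented as Dex.
; The montage's gameplay event triggers the projectile spawn from the tagged socket toward the target's current location, with optional pitch override.
; EndAbility and MontageStop nodes are unconnected.
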(event `self.K2_ActivateAbility`
  (bind _returnvalue (`self.GetAvatarActorFromActorInfo`))
  (bind _returnvalue_2 (`self.GetAvatarActorFromActorInfo`))
  ;[0.09549 0.4203 1] Get Target and Facing Rotation
  (bind _returnvalue_3 (message `EnemyInterface.GetCombatTarget` _returnvalue_2))
  (bind _ascombat_interface (cast `CombatInterface` _returnvalue_2))
  (message `CombatInterface.UpdateFacingTarget` (`KismetSystemLibrary.Conv_InterfaceToObject` _ascombat_interface) (`Actor.K2_GetActorLocation` _returnvalue_3))
  ;[0.1345 0.09615 1] Get montages and pick one from random
  (bind _returnvalue_4 (message `CombatInterface.GetAttackMontages` (`self.GetAvatarActorFromActorInfo`)))
  (bind _output_get (set `self.TaggedMontage` (`self.GetRandomTaggedMontageFromArray` _returnvalue_4)))
  (bind (_montage _montagetag _sockettag) (break `TaggedMontage` _output_get))
  (`AbilityTask_PlayMontageAndWait.CreatePlayMontageAndWaitProxy` "None" _montage (+ (/ (`.ReturnValue` (`AbilitySystemComponent.GetGameplayAttributeValue` (`AbilitySystemBlueprintLibrary.GetAbilitySystemComponent` (`self.GetAvatarActorFromActorInfo`)) (struct :`AttributeName` "Dexterity" :`Attribute` "/Script/LabyrinthUE53.LabyrinthAttributeSet:Dexterity" :`AttributeOwner` "/Script/CoreUObject.Class'/Script/LabyrinthUE53.LabyrinthAttributeSet'"))) 100.0) 1.0)
    (:`then`
      (`AbilityTask_WaitGameplayEvent.WaitGameplayEvent` _montagetag null true
        (:`EventReceived`
          (message `CombatInterface.GetCombatSocketLocation` _returnvalue _sockettag)
          (bind _returnvalue_5 (message `EnemyInterface.GetCombatTarget` _returnvalue))
          (`self.SpawnProjectile` (`Actor.K2_GetActorLocation` _returnvalue_5) _sockettag (`self.ShouldOverridePitch`) (`self.PitchOverride`)))))))