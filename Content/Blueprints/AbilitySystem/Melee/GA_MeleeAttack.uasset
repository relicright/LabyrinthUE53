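; Melee attack gameplay ability that plays an attack montage and deals damage around the avatar's combat socket.
; It turns off cursor facing until the montage's attack event arrives, then restores it and adds a loose secondary melee tag.
; That event triggers a radius query for live players, applying damage with upward knockback and drawing a debug sphere.
; The ability ends shortly after the montage finishes or is interrupted, removing the tag.
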(event `self.K2_ActivateAbility`
  (bind _returnvalue (`self.GetAvatarActorFromActorInfo`))
  (set `self.HasHitTarget` false)
  ;[1 1 1] Commit Cooldown and Cost
  (`self.K2_CommitAbility`)
  ;[1 1 1] Play the montage and wait for the AN_MontageEvent
  (`AbilityTask_PlayMontageAndWait.CreatePlayMontageAndWaitProxy` "None" "/Game/Assets/Animations/Character/OneHandedSword/AM_MeleeAttackTest.AM_MeleeAttackTest" 0.75
    (:`then`
      (bind _output_get (set `self.AvatarActor` (`self.GetAvatarActorFromActorInfo`)))
      (bind _aslabyrinth_character (cast `LabyrinthCharacter` _output_get))
      (`LabyrinthCharacter.SetShouldFaceMouseCursor` _aslabyrinth_character false)
      (`AbilityTask_WaitGameplayEvent.WaitGameplayEvent` (struct :`TagName` "Abilities.Attack") null
        (:`EventReceived`
          (`LabyrinthCharacter.SetShouldFaceMouseCursor` _aslabyrinth_character true)
          (`AbilitySystemBlueprintLibrary.AddLooseGameplayTags` _returnvalue (`BlueprintGameplayTagLibrary.MakeGameplayTagContainerFromArray` (`|MakeArray` (`self.MeleeSecondaryTag`))))
          (bind _returnvalue_2 (message `CombatInterface.GetCombatSocketLocation` _returnvalue (`BlueprintGameplayTagLibrary.MakeLiteralGameplayTag` (struct :`TagName` "Abilities.Attack"))))
          (`KismetSystemLibrary.DrawDebugSphere` _returnvalue_2 120.0 12 (struct :`R` 1.0 :`G` 1.0 :`B` 1.0 :`A` 1.0) 5.0 3.0)
          ;[1 0.1009 0] Causes Error from combatInterface
          (bind _outoverlappingactors (`LabyrinthAbilitySystemLibrary.GetLivePlayersWithinRadius` _returnvalue (`|MakeArray` _returnvalue) 100.0 _returnvalue_2))
          (for _array_element _outoverlappingactors
            (`LabyrinthAbilitySystemLibrary.ApplyDamageEffect` (`self.MakeDamageEffectParamsFromClassDefaults` _array_element (0.0 0.0 0.0) true (0.0 0.0 10000.0)))
            (set `self.HasHitTarget` true)))))
    (:`OnCompleted`
      (`KismetSystemLibrary.Delay` 0.2 :!label _label)
      (`self.K2_EndAbility`))
    (:`OnBlendOut`
      (goto _label))
    (:`OnInterrupted`
      (goto _label))
    (:`OnCancelled`
      (goto _label))))

(event `self.K2_OnEndAbility`
  (params (bWasCancelled :type Boolean))
  (`AbilitySystemBlueprintLibrary.RemoveLooseGameplayTags` (`self.GetAvatarActorFromActorInfo`) (`BlueprintGameplayTagLibrary.MakeGameplayTagContainerFromArray` (`|MakeArray` (`self.MeleeSecondaryTag`)))))

(fn `RemoveLooseTags`
  (`AbilitySystemBlueprintLibrary.RemoveLooseGameplayTags` (`self.AvatarActor`) (`BlueprintGameplayTagLibrary.MakeGameplayTagContainerFromArray` (`|MakeArray` (`self.MeleeSecondaryTag`))) true))