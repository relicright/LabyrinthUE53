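; Shield Knight skeleton enemy Blueprint that supports turning toward a target through Motion Warping.
; UpdateFacingTarget sets the FacingTarget warp location unless the Dead flag is set.
; IsDead always returns false rather than reading that flag.
; The construction script only calls its parent, and BeginPlay, overlap and Tick are disabled stubs.
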(event `CombatInterface.UpdateFacingTarget`
  (params (Target :type "Vector Structure (by ref)"))
  (if (not (`self.bDead`))
    (`MotionWarpingComponent.AddOrUpdateWarpTargetFromLocation` (`self.MotionWarping`) "FacingTarget" Target)))

(fn `IsDead`
  (returns (ReturnValue :type Boolean))
  (return false))

(fn `UserConstructionScript`
  (`parent.UserConstructionScript`))